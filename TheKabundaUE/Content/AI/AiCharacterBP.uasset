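; Enemy AI character that starts roaming, patrolling or chasing based on AiState and switches to chasing the player on sight via PawnSensing.
; Roam and Patrol loop latent AIMoveTo calls, using random nearby points or target points.
; ChasePlayer reissues moves and applies damage each second without waiting for arrival, while sensing is enabled.
; Player death or its own lethal damage triggers ResetAI, disabling sensing; dead AI is destroyed after a delay.
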(event `ResetAI`
  (`PawnSensingComponent.SetSensingUpdatesEnabled` (`self.PawnSensing`) false)
  (switch `/Game/AI/AiState` (`self.AiState`)
    (:`NewEnumerator1`
      (`self.Roam`))
    (:`NewEnumerator3`
      (`self.Patrol`))
    (:`NewEnumerator2`
      (`self.ChasePlayer` null))
    (:`NewEnumerator5`
      (`KismetSystemLibrary.Delay` 10.0)
      (`self.K2_DestroyActor`))))

(event `self.ReceiveBeginPlay`
  (bind _astop_down_character (cast `/Game/TopDownCPP/Blueprints/TopDownCharacter` (`GameplayStatics.GetPlayerPawn` 0)))
  (add `/Game/TopDownCPP/Blueprints/TopDownCharacter.PlayerDied` _astop_down_character (delegate `ResetAI`))
  ;[1 1 1] Select Starting state
  (switch `/Game/AI/AiState` (`self.AiState`)
    (:`NewEnumerator1`
      (`self.Roam`))
    (:`NewEnumerator3`
      (`self.Patrol`))
    (:`NewEnumerator2`
      (`self.ChasePlayer` (`GameplayStatics.GetPlayerPawn` 0)))))

(event `Roam`
  ;[1 1 1] AI Roam
  (`|AIMoveTo` self (`NavigationSystem.GetRandomPointInNavigableRadius` (`self.K2_GetActorLocation`) 200.0) null 5.0
    (:`OnSuccess`
      (`KismetSystemLibrary.Delay` 4.0)
      (`self.Roam`))))

(event `self.PawnSensing.OnSeePawn`
  (params (Pawn :type "Pawn Object Reference"))
  ;[1 1 1] Chase player on seen
  (if (not (`self.IsChasing`))
    (set `self.IsChasing` true)
    (bind _astop_down_character (cast `/Game/TopDownCPP/Blueprints/TopDownCharacter` Pawn))
    (`self.ChasePlayer` _astop_down_character)))

(event `ChasePlayer`
  (params (ActorToChase :type "Pawn Object Reference"))
  ;[1 1 1] Chase Player
  (if (`PawnSensingComponent.bEnableSensingUpdates` (`self.PawnSensing`))
    (`|AIMoveTo` self (0.0 0.0 0.0) ActorToChase
      (:`then`
        (`GameplayStatics.ApplyDamage` ActorToChase (`self.Damage`))
        (`KismetSystemLibrary.Delay` 1.0)
        (`self.ChasePlayer` ActorToChase)))))

(event `Patrol`
  ;[1 1 1] Patrol
  (`self.IsOnPatrol`)
  (`|AIMoveTo` self (0.0 0.0 0.0) (`self.TargetPoint1`) 5.0
    (:`OnSuccess`
      (`KismetSystemLibrary.Delay` 4.0)
      (`self.IsOnPatrol`)
      (`|AIMoveTo` self (0.0 0.0 0.0) (`self.TargetPoint2`)
        (:`OnSuccess`
          (`KismetSystemLibrary.Delay` 4.0)
          (`self.Patrol`))))))

(event `self.ReceiveAnyDamage`
  (params (Damage :type "Float (single-precision)") (DamageType :type "DamageType Object Reference") (InstigatedBy :type "Controller Object Reference") (DamageCauser :type "Actor Object Reference"))
  (bind _mesh (`self.Mesh`))
  ;[1 1 1] On Damage Event
  (bind _output_get (set `self.CurrentHealth` (- (`self.CurrentHealth`) Damage)))
  (if (and (<= _output_get 0.0) (`|EnumInequality` (`self.AiState`) "NewEnumerator5"))
    (`SkeletalMeshComponent.PlayAnimation` _mesh "/Game/Mannequin/Animations/SwordAndShield/death.death" false)
    (`GameplayStatics.PlaySoundAtLocation` "/Game/Sounds/Death2_Cue.Death2_Cue" (`SceneComponent.GetSocketLocation` _mesh "None"))
    (set `self.AiState` "NewEnumerator5")
    (`self.ResetAI`)))

(fn `UserConstructionScript`)